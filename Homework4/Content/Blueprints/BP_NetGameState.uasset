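; Networked game state Blueprint that handles the end and restart of a team match.
; On victory it loops over the player array and calls won on Red team avatars and lost on Blue ones, so Red is always treated as the winner.
; ShowResultMessage creates and displays the results widget, though its winner-name and lose-text logic is left unconnected.
; On restart it removes that widget from the screen.
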(event `self.OnVictory`
  (for _array_element (`self.PlayerArray`)
    (bind _asnet_player_state (cast `NetPlayerState` _array_element))
    (switch `EPlayerTeam` (`.Team` (break `SPlayerInfo` (`NetPlayerState.PlayerInfo` _asnet_player_state)))
      (:`TEAM_Blue`
        (bind _asbp_avatar (cast `/Game/Blueprints/BP_Avatar` (`PlayerState.PawnPrivate` _asnet_player_state) :!pure true))
        (`/Game/Blueprints/BP_Avatar.OnPlayerLost` _asbp_avatar))
      (:`TEAM_Red`
        (`/Game/Blueprints/BP_Avatar.OnPlayerWon` _asbp_avatar)))))

(event `self.OnRestart`
  (`Widget.RemoveFromParent` (`self.MessageWidget`)))

(fn `ShowResultMessage`
  (bind _returnvalue (`self.GetPlayerStateByIndex` (`self.WinningPlayer`)))
  (bind _returnvalue_2 (`|CreateWidget` "/Game/Blueprints/UMG/W_Game_Results.W_Game_Results_C"))
  (set `self.MessageWidget` _returnvalue_2)
  (`UserWidget.AddToViewport` _returnvalue_2 0))

(fn `UserConstructionScript`)